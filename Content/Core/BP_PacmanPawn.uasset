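; Player Pac-Man pawn that enables movement after a start delay and manages the HUD, pause and end-game screens.
; Timelines smooth rotation along the shortest path and, on death, disable collision and ease speed to zero before showing the loss screen.
; The game mode's win event shows the same end screen as a win, with input disabled.
; Input also toggles the pause menu, reloads the level or quits.
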(event `self.ReceiveBeginPlay`
  ;[1 1 1] Initialize and Bind
  (`KismetSystemLibrary.Delay` 4.0)
  (set `self.bCanMove` true)
  (bind _returnvalue (`|CreateWidget` "/Game/Core/WBP_Score.WBP_Score_C" (`GameplayStatics.GetPlayerController` 0)))
  (`UserWidget.AddToViewport` _returnvalue 0)
  (bind _aslm_pacman_gm (cast `LM_Pacman_GM` (`GameplayStatics.GetGameMode`)))
  (add `LM_Pacman_GM.OnPlayerWin` _aslm_pacman_gm (delegate `OnPlayerWin_Event_0`)))

(event `OnPlayerWin_Event_0`
  ;[1 1 1] Initialize and Bind
  (`self.EndGameUI` true))

(event `self.SmoothSetRotation`
  (params (DesiredRotation :type "Rotator Structure"))
  ;[1 1 1] Smooth Rotate
  (set `self.InitRotation` (`self.K2_GetActorRotation`))
  (bind (_direction _alpha) (`Timeline|Timeline_SmoothRotation` :!via `PlayFromStart`)
    (:`Update`
      (`self.K2_SetActorRotation` (`KismetMathLibrary.RLerp` (`self.InitRotation`) DesiredRotation _alpha true) true))))

(event `self.Die`
  ;[1 1 1] Die
  (`parent.Die`)
  (set `self.StoredMaxSpeed` (`MovementComponent.GetMaxSpeed` (`self.FloatingPawnMovementComponent`)))
  (`PrimitiveComponent.SetCollisionEnabled` (`self.SphereComp`) "NoCollision")
  (bind (_direction _alpha) (`Timeline|Timeline_MovementSpeed` :!via `PlayFromStart`)
    (:`Update`
      (set `FloatingPawnMovement.MaxSpeed` (`KismetMathLibrary.Lerp` (`self.StoredMaxSpeed`) 0.0 _alpha) (`self.FloatingPawnMovementComponent`)))
    (:`Finished`
      (`self.EndGameUI` false))))

(event `EndGameUI`
  (params (bWin :type Boolean))
  ;[1 1 1] End Game
  (bind _returnvalue (`|CreateWidget` "/Game/Core/WBP_EndGame.WBP_EndGame_C" null bWin))
  (`UserWidget.AddToViewport` _returnvalue 0)
  (`self.DisableInput` (`GameplayStatics.GetPlayerController` 0)))

(event `InputAction|Pause`
  (params (Key :type "Key Structure"))
  ;[1 1 1] Pause Game
  (:`Pressed`
    (bind _isa (`/Engine/EditorBlueprintResources/StandardMacros.FlipFlop`)
      (:`A`
        _)
      (:`B`
        _))
    (bind _returnvalue (`GameplayStatics.SetGamePaused` _isa))
    (if _returnvalue
      (bind _returnvalue_2 (`|CreateWidget` "/Game/Core/WBP_Pause.WBP_Pause_C" (`GameplayStatics.GetPlayerController` 0)))
      (`UserWidget.AddToViewport` _returnvalue_2 0)
      (set `self.PauseMenu` _returnvalue_2)
      (else
        (`Widget.RemoveFromParent` (`self.PauseMenu`))))))

(event `Key|R` :paused true
  (params (Key :type "Key Structure"))
  ;[1 1 1] Pause Game
  (:`Pressed`
    (if (stale `InputAction|Pause` _returnvalue)
      (bind _returnvalue (`GameplayStatics.GetCurrentLevelName` true))
      (`GameplayStatics.OpenLevel` (`KismetStringLibrary.Conv_StringToName` _returnvalue)))))

(event `InputAction|Quit`
  (params (Key :type "Key Structure"))
  ;[1 1 1] Quit Game
  (:`Pressed`
    (`KismetSystemLibrary.QuitGame` null "Quit")))

(fn `UserConstructionScript`)