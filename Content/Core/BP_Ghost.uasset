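; BP_Ghost is a ghost pawn with floating movement that calls GameStart four seconds after BeginPlay.
; Timeline-driven events smoothly rotate it or return it to its spawn location facing forward, then toggle eye and mesh visibility.
; Speed changes blend max speed through a timeline, with an optional timer that reverses the timeline to restore the previous speed.
; The construction script applies the ghost's color to its mesh materials.
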(event `self.ReceiveBeginPlay`
  (`KismetSystemLibrary.Delay` 4.0)
  (`self.GameStart`))

(event `self.SetRotationSmoothly`
  (params (DesiredRotation :type "Rotator Structure"))
  ;[1 1 1] Update Movement Rotation
  (set `self.StoredRotation` (`self.K2_GetActorRotation`))
  (bind (_direction _alpha) (`Timeline|Timeline_SetRotationSmoothly` :!via `PlayFromStart`)
    (:`Update`
      (`self.K2_SetActorRotation` (`KismetMathLibrary.RLerp` (`self.StoredRotation`) DesiredRotation _alpha true) true))))

(event `self.SetIdleLocationAndRotationSmoothly`
  (bind (_returnvalue_location _returnvalue_rotation) (`KismetMathLibrary.BreakTransform` (`self.GetTransform`)))
  ;[1 1 1] Reset Ghost Position
  (set `self.StoredLocation` _returnvalue_location)
  (set `self.StoredRotation` _returnvalue_rotation)
  (bind (_direction _alpha) (`Timeline|Timeline_SetLoc&Rot` :!via `PlayFromStart`)
    (:`Update`
      (`self.K2_SetActorLocationAndRotation` (`KismetMathLibrary.VLerp` (`self.StoredLocation`) (`self.SpawnLocation`) _alpha) (`KismetMathLibrary.RLerp` (`self.StoredRotation`) (`KismetMathLibrary.MakeRotFromX` (`KismetMathLibrary.Vector_Forward`)) _alpha true)))
    (:`Finished`
      (`SceneComponent.ToggleVisibility` (`self.GhostEye`) false)
      (`SceneComponent.ToggleVisibility` (`self.GhostMesh`) false))))

(event `self.SetMovementSpeedSmoothly`
  (params (NewSpeed :type "Float (single-precision)") (ResetDelay :type "Float (single-precision)"))
  ;[1 1 1] Update Movespeed and Reset Back if Delay > 0
  (`|ExecutionSequence`
    (:`then_0`
      (`KismetSystemLibrary.K2_ClearAndInvalidateTimerHandle` (`self.TimerHandle_ResetMovement`))
      (if (> ResetDelay 0.0)
        (bind _returnvalue (`KismetSystemLibrary.K2_SetTimerDelegate` (delegate `ResetMovementSpeed`) ResetDelay))
        (set `self.TimerHandle_ResetMovement` _returnvalue)))
    (:`then_1`
      (set `self.StoredMovement` (`MovementComponent.GetMaxSpeed` (`self.FloatingPawnMovementComponent`)))
      (`TimelineComponent.SetPlayRate` (`self.Timeline_SetMovementSpeedSmoothly`) (/ 1.0 (`self.TimeToFullyUpdateMovementSpeed`)))
      (bind (_direction _alpha) (`Timeline|Timeline_SetMovementSpeedSmoothly` :!via `PlayFromStart` :!label _label)
        (:`Update`
          (set `FloatingPawnMovement.MaxSpeed` (`KismetMathLibrary.Lerp` (`self.StoredMovement`) NewSpeed _alpha) (`self.FloatingPawnMovementComponent`)))))))

(event `ResetMovementSpeed`
  ;[1 1 1] Update Movespeed and Reset Back if Delay > 0
  (goto _label :!via `Reverse`))

(fn `UserConstructionScript`
  (`MeshComponent.SetVectorParameterValueOnMaterials` (`self.GhostMesh`) "GhostColor" (`self.GhostColor`)))